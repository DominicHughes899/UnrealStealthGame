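; BP_DisappearingText is a short-lived floating text actor that shows a given string in a given colour.
; On BeginPlay it applies the text, colour and a fixed world rotation to its TextRender component.
; Each Tick it accumulates a timer, moves the text along its local Z at RiseRate, and destroys itself once the timer reaches LifeTime.
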(event EventBeginPlay
  (bind _textrender (Variables|Default|GetTextRender))
  (Rendering|Components|TextRender|SetText _textrender (Variables|Default|GetTextToDisplay))
  (Rendering|Components|TextRender|SetTextRenderColor _textrender (Variables|Default|GetTextColour))
  (Transformation|SetWorldRotation (Variables|Default|GetTextRender) "20.000000,180.000000,0.000000" false false))

(event EventTick
  (params (DeltaSeconds :type Float%20%28single-precision%29))
  (CallFunction|UpdateTimer DeltaSeconds)
  (CallFunction|Animate DeltaSeconds)
  (CallFunction|DestroyifOld))

(fn ConstructionScript)

(fn UpdateTimer
  (params (DeltaTime :type Float%20%28double-precision%29))
  (Variables|Default|SetTimer (+ DeltaTime (Variables|Default|GetTimer))))

(fn Animate
  (params (DeltaTime :type Float%20%28double-precision%29))
  (Transformation|AddLocalOffset (Variables|Default|GetTextRender) (Math|Vector|MakeVector 0.0 0.0 (* DeltaTime (Variables|Default|GetRiseRate))) false false))

(fn DestroyifOld
  (if (>= (Variables|Default|GetTimer) (Variables|Default|GetLifeTime))
    (Actor|DestroyActor)))