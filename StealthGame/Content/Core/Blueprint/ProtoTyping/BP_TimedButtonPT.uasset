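; Prototype timed button that gives visual feedback for press, countdown, timeout and locked states.
; Pressing shifts the Cylinder along its local Z axis, and timeout shifts it back and prints a debug message.
; Counter changes and locked attempts spawn BP_DisappearingText at the button, showing the current count or a keycard-required notice.
; The graph only handles these events; the timer and lock logic are not in it.
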(event EventOnLocked
  (Game|SpawnActorfromClass "/Game/Core/Blueprint/MiscText/BP_DisappearingText.BP_DisappearingText_C" (Transformation|GetActorTransform) "Undefined" 0 "KeyCard Required" (Variables|Default|GetText%20Colour) 0))

(event EventOnCounterChanged
  (params (CounterNumber :type Integer))
  (Game|SpawnActorfromClass "/Game/Core/Blueprint/MiscText/BP_DisappearingText.BP_DisappearingText_C" (Transformation|GetActorTransform) "Undefined" 0 (Utilities|Text|ToText(Integer) CounterNumber) (Variables|Default|GetText%20Colour) 0))

(event EventOnPressed
  (Transformation|AddLocalOffset (Variables|Default|GetCylinder) "0.000000,0.000000,20.000000" false false))

(event EventOnTimeout
  (Development|PrintString "Ended")
  (Transformation|AddLocalOffset (Variables|Default|GetCylinder) "0.000000, 0,-20.000000" false false))

(fn ConstructionScript)