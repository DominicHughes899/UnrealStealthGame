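; Prototype light-plate actor that cycles four rect lights through a fixed chase pattern with switch clicks.
; A looping one-second timer advances a step counter, whose branch chain toggles lights so one replaces the next, then pauses dark before repeating.
; Each light's FlipFlop drives its visibility and plays an attenuated click at the actor when it turns on.
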(event Custom|Toggle%20Light%204
  (bind _isa (Utilities|FlowControl|FlipFlop)
    (:A
      _)
    (:B
      _))
  (Rendering|SetVisibility (Variables|Default|GetRectLight4) _isa false)
  (if _isa
    (Audio|SpawnSoundatLocation "/Game/Core/Audio/SFX/Wav/Button_Switch.Button_Switch" (Transformation|GetActorLocation) "0, 0, 0" 1e+01 1.0 0.0 "/Game/Core/Audio/SFX/Attenuation/ClickAttenuation.ClickAttenuation" 0)))

(event Custom|Toggle%20Light%202
  (bind _isa (Utilities|FlowControl|FlipFlop)
    (:A
      _)
    (:B
      _))
  (Rendering|SetVisibility (Variables|Default|GetRectLight2) _isa false)
  (if _isa
    (Audio|SpawnSoundatLocation "/Game/Core/Audio/SFX/Wav/Button_Switch.Button_Switch" (Transformation|GetActorLocation) "0, 0, 0" 1e+01 1.0 0.0 "/Game/Core/Audio/SFX/Attenuation/ClickAttenuation.ClickAttenuation" 0)))

(event Custom|Toggle%20Light
  (Variables|Default|SetLight%20State (+ (Variables|Default|GetLight%20State) 1))
  (if (== (Variables|Default|GetLight%20State) 1)
    (CallFunction|ToggleLight3)
    (elif (== (Variables|Default|GetLight%20State) 2)
      (CallFunction|ToggleLight3)
      (CallFunction|ToggleLight4)
      (elif (== (Variables|Default|GetLight%20State) 3)
        (CallFunction|ToggleLight4)
        (CallFunction|ToggleLight1)
        (elif (== (Variables|Default|GetLight%20State) 4)
          (CallFunction|ToggleLight1)
          (CallFunction|ToggleLight2)
          (elif (== (Variables|Default|GetLight%20State) 5)
            (CallFunction|ToggleLight2)
            (CallFunction|ToggleLight1)
            (elif (== (Variables|Default|GetLight%20State) 6)
              (CallFunction|ToggleLight1)
              (CallFunction|ToggleLight3)
              (elif (== (Variables|Default|GetLight%20State) 7)
                (CallFunction|ToggleLight3)
                (elif (== 8 (Variables|Default|GetLight%20State))
                  (Variables|Default|SetLight%20State 0))))))))))

(event Custom|Toggle%20Light%201
  (bind _isa (Utilities|FlowControl|FlipFlop)
    (:A
      _)
    (:B
      _))
  (Rendering|SetVisibility (Variables|Default|GetRectLight1) _isa false)
  (if _isa
    (Audio|SpawnSoundatLocation "/Game/Core/Audio/SFX/Wav/Button_Switch.Button_Switch" (Transformation|GetActorLocation) "0, 0, 0" 1e+01 1.0 0.0 "/Game/Core/Audio/SFX/Attenuation/ClickAttenuation.ClickAttenuation" 0)))

(event Custom|Toggle%20Light%203
  (bind _isa (Utilities|FlowControl|FlipFlop)
    (:A
      _)
    (:B
      _))
  (Rendering|SetVisibility (Variables|Default|GetRectLight3) _isa false)
  (if _isa
    (Audio|SpawnSoundatLocation "/Game/Core/Audio/SFX/Wav/Button_Switch.Button_Switch" (Transformation|GetActorLocation) "0, 0, 0" 1e+01 1.0 0.0 "/Game/Core/Audio/SFX/Attenuation/ClickAttenuation.ClickAttenuation" 0)))

(event EventBeginPlay
  (Utilities|Time|SetTimerbyEvent (delegate Custom|Toggle%20Light) 1.0 true))

(fn ConstructionScript)