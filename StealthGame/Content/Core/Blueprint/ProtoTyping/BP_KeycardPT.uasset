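; BP_KeycardPT is a prototype keycard pickup that spins and bobs in the world.
; Tick runs AnimateKeyCard, which yaws the mesh by RotationRate and adds a sine-driven Z offset each frame, so bob height depends on frame rate.
; On successful interaction it hides the Plane component and plays an acquired sound; on failure it spawns red "Hands Full" disappearing text.
; The Unlock event is empty.
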(event EventBeginPlay)

(event Collision|EventActorBeginOverlap
  (params (OtherActor :type Actor%20Object%20Reference)))

(event EventTick
  (params (DeltaSeconds :type Float%20%28single-precision%29))
  (CallFunction|AnimateKeyCard DeltaSeconds))

(event EventOnInteracted
  (params (Success :type Boolean))
  (if Success
    (Rendering|SetVisibility (Variables|Default|GetPlane) false false)
    (Audio|PlaySound2D "/Game/Core/Audio/SFX/Wav/Object_Acquired.Object_Acquired" 1.0 1.0 0.0 0 0)
    (else
      (Game|SpawnActorfromClass "/Game/Core/Blueprint/MiscText/BP_DisappearingText.BP_DisappearingText_C" (Transformation|GetActorTransform) "Undefined" 0 "Hands Full :(" (Math|Color|MakeColor 0 0 255) 0))))

(event EventUnlock)

(fn ConstructionScript)

(fn AnimateKeyCard
  (params (DeltaTime :type Float%20%28double-precision%29))
  (Transformation|AddLocalRotation (Variables|Default|GetSM_KeyCard) (Math|Rotator|MakeRotator 0.0 0.0 (* (Variables|Default|GetRotationRate) DeltaTime)) false false)
  (bind _output_get (Variables|Default|SetTimer (+ (Variables|Default|GetTimer) DeltaTime)))
  (Transformation|AddLocalOffset (Variables|Default|GetSM_KeyCard) (Math|Vector|MakeVector 0.0 0.0 (/ (Math|Trig|Sin(Radians) (* _output_get 2.0)) 2.0)) false false))