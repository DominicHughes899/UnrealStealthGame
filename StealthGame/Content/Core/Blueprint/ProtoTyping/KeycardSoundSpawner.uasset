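; Prototype musical puzzle Blueprint that reveals a keycard when pressure plates are pressed in the correct note order.
; AddNote reads the note from the recently pressed BP_PressurePlate into a rolling six-entry history.
; When that history matches CorrectSequence, it makes the existing keycard visible and plays a success sound.
; KeycardSpawned gates the logic but is only assigned to itself, so the match never latches it.
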(event Custom|Add%20Note
  (bind _recently_played_notes (Variables|Default|GetRecently%20Played%20Notes))
  (if (not (Variables|Default|GetKeycard%20Spawned))
    (bind _asbp_pressure_plate (Utilities|Casting|CastToBP_PressurePlate (Variables|Default|GetRecently%20Pressed%20Plate)))
    (if (>= (Utilities|Array|Length _recently_played_notes) 6)
      (Utilities|Array|RemoveIndex _recently_played_notes))
    (Utilities|Array|Add _recently_played_notes (Variables|/Game/Core/Blueprint/ProtoTyping/BP_PressurePlate.BP_PressurePlate_C|GetNote _asbp_pressure_plate))
    (if (Utilities|Array|Identical (Variables|Default|GetRecently%20Played%20Notes) (Variables|Default|GetCorrect%20Sequence))
      (Rendering|SetVisibility (Variables|Default|GetBP_KeycardPT) true false)
      (Audio|PlaySound2D "/Game/Core/Audio/SFX/Wav/Success.Success" 1.0 1.0 0.0 0 0)
      (Variables|Default|SetKeycard%20Spawned (Variables|Default|GetKeycard%20Spawned)))))

(fn ConstructionScript)