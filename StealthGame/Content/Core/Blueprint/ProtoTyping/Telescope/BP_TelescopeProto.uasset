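; Prototype interactable telescope that the top-down player controller possesses to look through with a zoomed camera.
; After a short possession delay, Tick drives a reversible timer that lerps camera FOV to zoom in, then reveals the telescope widget.
; While possessed, movement axes rotate the telescope mesh.
; StopLooking hides the widget, reverses the zoom, and has the controller repossess the character.
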(event Custom|Event%20StopLooking
  (Widget|SetVisibility (Variables|Default|GetTelescopeUI) "Hidden")
  (Variables|Default|SetShouldUnzoom true)
  (Utilities|FlowControl|Delay (Variables|Default|GetZoomTime))
  (bind _asbp_top_down_player_controller (Utilities|Casting|CastToBP_TopDownPlayerController (Variables|Default|GetPlayer%20Controller)))
  (Default|EventRePossessCharacter _asbp_top_down_player_controller)
  (Camera|SetFieldOfView (Variables|Default|GetCamera) 9e+01))

(event EventMoveForward
  (params (Value :type Float%20%28single-precision%29))
  (Transformation|AddLocalRotation (Variables|Default|GetSM_Telescope) (Math|Rotator|MakeRotator (* Value (Variables|Default|GetMoveSpeed)) 0.0 0.0) false false))

(event EventTick
  (params (DeltaSeconds :type Float%20%28single-precision%29))
  (bind _timer (Variables|Default|GetTimer))
  (Utilities|FlowControl|Sequence
    (:then_0
      (if (Variables|Default|GetShouldZoom)
        (bind _output_get (CallFunction|UpdateTimer DeltaSeconds))
        (CallFunction|LerpFOV _output_get)
        (if (>= _timer (Variables|Default|GetZoomTime))
          (Variables|Default|SetShouldZoom false)
          (Variables|Default|SetReverseTimer true)
          (Widget|SetVisibility (Variables|Default|GetTelescopeUI) "Visible"))))
    (:then_1
      (if (Variables|Default|GetShouldUnzoom)
        (bind _output_get_2 (CallFunction|UpdateTimer DeltaSeconds))
        (CallFunction|LerpFOV _output_get_2)
        (if (<= _timer 0.0)
          (Variables|Default|SetShouldUnzoom false)
          (Variables|Default|SetReverseTimer false))))))

(event EventBeginPlay
  (bind _returnvalue (UserInterface|CreateWidget "/Game/Core/Blueprint/UI/Game/EBP_Telescope.EBP_Telescope_C" 0 self))
  (bind _output_get (Variables|Default|SetTelescopeUI _returnvalue))
  (Widget|SetVisibility _output_get "Hidden")
  (UserInterface|Viewport|AddtoViewport _output_get 0))

(event EventMoveRight
  (params (Value :type Float%20%28single-precision%29))
  (Transformation|AddLocalRotation (Variables|Default|GetSM_Telescope) (Math|Rotator|MakeRotator 0.0 0.0 (* Value (Variables|Default|GetMoveSpeed))) false false))

(event EventOnPlayerInteraction
  (params (PlayerController :type Player%20Controller%20Object%20Reference))
  (bind _output_get (Variables|Default|SetPlayer%20Controller PlayerController))
  (bind _asbp_top_down_player_controller (Utilities|Casting|CastToBP_TopDownPlayerController _output_get))
  (Development|PrintString "1")
  (Default|EventPossessPawn _asbp_top_down_player_controller self)
  (Utilities|FlowControl|Delay 1.1)
  (Variables|Default|SetShouldZoom true)
  (Development|PrintString "Possessed"))

(fn ConstructionScript)

(fn UpdateTimer
  (params (A :type Float%20%28double-precision%29))
  (if (Variables|Default|GetReverseTimer)
    (bind _output_get (Variables|Default|SetTimer (- (Variables|Default|GetTimer) A)))
    (else
      (Variables|Default|SetTimer (+ A (Variables|Default|GetTimer)))))
  (return _output_get))

(fn LerpFOV
  (params (A :type Float%20%28double-precision%29))
  (bind _zoomtime (Variables|Default|GetZoomTime))
  (bind _returnvalue (/ A _zoomtime))
  (bind _returnvalue_2 (Math|Float|Lerp 9e+01 2e+01 _returnvalue))
  (Development|PrintString (Utilities|String|ToString(Float) _returnvalue_2))
  (Camera|SetFieldOfView (Variables|Default|GetCamera) _returnvalue_2))