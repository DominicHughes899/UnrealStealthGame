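; BP_Interactable_Lever is an interactable lever whose handle rotates to reflect its LeverState boolean, with feedback when it is locked.
; BeginPlay pre-rotates the handle if the state is on, and LeverInteraction swings it either way by that state, printing On or Off.
; OnLocked spawns a red "Keycard Required" BP_DisappearingText at the lever and plays a 2D failure sound.
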(event EventBeginPlay
  (if (Variables|Default|GetLeverState)
    (Transformation|AddLocalRotation (Variables|Default|GetLeverHandle) "90.000000, 0, 0" false false)))

(event EventOnLocked
  (Game|SpawnActorfromClass "/Game/Core/Blueprint/MiscText/BP_DisappearingText.BP_DisappearingText_C" (Transformation|GetActorTransform) "Undefined" 0 "Keycard Required" (Math|Color|MakeColor 0 0 255) 0)
  (bind _returnvalue (Audio|CreateSound2D "/Engine/EditorSounds/Notifications/CompileFailed.CompileFailed" 1.0 1.0 0.0 0))
  (Audio|Components|Audio|Play _returnvalue 0.0))

(event EventLeverInteraction
  (bind _leverhandle (Variables|Default|GetLeverHandle))
  (if (Variables|Default|GetLeverState)
    (Development|PrintString "On")
    (Transformation|AddLocalRotation _leverhandle "90.000000, 0, 0" false false)
    (else
      (Development|PrintString "Off")
      (Transformation|AddLocalRotation _leverhandle "-90.000000, 0, 0" false false))))

(fn ConstructionScript)