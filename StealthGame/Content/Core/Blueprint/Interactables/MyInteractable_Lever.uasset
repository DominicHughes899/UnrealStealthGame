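; Interactable lever Blueprint whose handle rotates to reflect the LeverState flag.
; On BeginPlay, a true LeverState pre-rotates the LeverHandle component 90 degrees in local space.
; The LeverInteraction event reads the flag, prints On or Off, and rotates the handle 90 degrees in the matching direction.
; These graphs only read LeverState and never change it.
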(event EventBeginPlay
  (if (Variables|Default|GetLeverState)
    (Transformation|AddLocalRotation (Variables|Default|GetLeverHandle) "90.000000, 0, 0" false false)))

(event EventLeverInteraction
  (bind _leverhandle (Variables|Default|GetLeverHandle))
  (if (Variables|Default|GetLeverState)
    (Development|PrintString "On")
    (Transformation|AddLocalRotation _leverhandle "90.000000, 0, 0" false false)
    (else
      (Development|PrintString "Off")
      (Transformation|AddLocalRotation _leverhandle "-90.000000, 0, 0" false false))))

(fn ConstructionScript)