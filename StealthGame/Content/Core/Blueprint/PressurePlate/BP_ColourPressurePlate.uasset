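; BP_ColourPressurePlate is a pressure plate that changes colour each time it is triggered, flagging itself as a colour plate on BeginPlay.
; On trigger it plays a button sound and applies the material at the current counter index to the plate mesh as a new dynamic instance.
; The counter then increments and wraps to zero at the end of the material array, so the colours cycle in order.
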(event EventBeginPlay
  (Variables|Default|SetIsColourPlate true))

(event EventOnPressurePlateTriggered
  (bind _materialarray (Variables|Default|GetMaterialArray))
  (Audio|PlaySound2D "/Game/Core/Audio/SFX/SoundCues/SC_Button.SC_Button" 1.0 1.0 0.0 0 0)
  (Rendering|Material|CreateDynamicMaterialInstance (Variables|Default|GetPlate) 0 (Utilities|Array|Get(acopy) _materialarray (Variables|Default|GetCounter)) "None" :!class /Script/Engine.PrimitiveComponent)
  (bind _result (Math|Integer|IncrementInt (Variables|Default|GetCounter))
    (:%20%20
      (if (== _result (Utilities|Array|Length _materialarray))
        (Variables|Default|SetCounter 0)))))

(fn ConstructionScript)