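; BP_SlidingDoor is an interactee double door that, despite its name, swings its two leaves open and closed by rotating them on yaw.
; A state change enables actor tick, and each tick AnimateDoors steps DoorR and DoorL in opposite directions toward open or closed based on Activated, at OpenSpeed.
; AnimateDoors returns a Finished flag, which switches tick off so the actor only ticks while animating.
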(event EventOnStateChange
  ;[1 1 1] Only enable tick when animating
  (Actor|Tick|SetActorTickEnabled true))

(event EventBeginPlay)

(event EventTick
  (params (DeltaSeconds :type Float%20%28single-precision%29))
  (bind _animationfinished (CallFunction|AnimateDoors DeltaSeconds))
  ;[1 1 1] Disable tick if animation finished
  (if _animationfinished
    (Actor|Tick|SetActorTickEnabled false)))

(fn ConstructionScript)

(fn AnimateDoors
  (params (DeltaTime :type Float%20%28double-precision%29))
  (bind _doorl (Variables|Default|GetDoorL))
  (bind _doorr (Variables|Default|GetDoorR))
  (bind _openspeed (Variables|Default|GetOpenSpeed))
  (bind _doorr_2 (Variables|Default|GetDoorR))
  (bind _doorl_2 (Variables|Default|GetDoorL))
  (bind _openspeed_2 (Variables|Default|GetOpenSpeed))
  (bind _returnvalue (* DeltaTime _openspeed))
  (bind _returnvalue_2 (* DeltaTime _openspeed_2))
  (bind _relativerotation (Variables|/Script/Engine.SceneComponent|GetRelativeRotation _doorr))
  (bind _relativerotation_2 (Variables|/Script/Engine.SceneComponent|GetRelativeRotation _doorl))
  (Utilities|FlowControl|Sequence
    (:then_0
      ;[1 1 1] Right Door
      (if (Variables|Default|GetActivated)
        ;;[1 0 0] Check if animation is needed
        (if (<= (.yaw _relativerotation) 9e+01)
          (Transformation|AddLocalRotation _doorr_2 (Math|Rotator|MakeRotator 0.0 0.0 _returnvalue) false false)
          ;[0.03475 1 0] Update Finished Flag
          (LocalVariables|SetFinished false :!label _label))
        (elif (>= (.yaw _relativerotation) 0.0)
          (Transformation|AddLocalRotation _doorr_2 (Math|Rotator|MakeRotator 0.0 0.0 (* _returnvalue -1.0)) false false)
          (goto _label))))
    (:then_1
      ;[1 1 1] Left Door
      (if (Variables|Default|GetActivated)
        ;;[1 0 0] Check if animation is needed
        (if (>= (.yaw _relativerotation_2) -9e+01)
          (Transformation|AddLocalRotation _doorl_2 (Math|Rotator|MakeRotator 0.0 0.0 (* _returnvalue_2 -1.0)) false false)
          (goto _label))
        (elif (<= (.yaw _relativerotation_2) 0.0)
          (Transformation|AddLocalRotation _doorl_2 (Math|Rotator|MakeRotator 0.0 0.0 _returnvalue_2) false false)
          (goto _label))))
    (:then_2
      ;[0 1 0.103] Return Animation finished Flag
      (return (LocalVariables|GetFinished)))))